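; BP_GameMode is a game mode that shows the game UI and keeps a score that rises with elapsed time.
; On BeginPlay it creates a BP_UI widget and adds it to the viewport.
; Tick accumulates delta time in a timer, adding one point to Score and resetting the timer each time it reaches a fixed two-second threshold.
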(event `self.ReceiveBeginPlay`
  (bind _returnvalue (`|CreateWidget` "/Game/BluePrint/BP_UI.BP_UI_C"))
  (`UserWidget.AddToViewport` _returnvalue 0))

(event `self.ReceiveTick`
  (params (DeltaSeconds :type "Float (single-precision)"))
  (bind _output_get (set `self.Timer` (+ DeltaSeconds (`self.Timer`))))
  (if (>= _output_get 2.0)
    (set `self.Score` (+ (`self.Score`) 1))
    (set `self.Timer` 0.0)))

(fn `UserConstructionScript`)