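; BP_Player is the player-controlled Blueprint that moves by Enhanced Input and fires missiles.
; BeginPlay adds the IMC_PlayerInput mapping context, and IA_Move sets a normalized 2D direction that Tick applies as an unswept location offset scaled by MoveSpeed.
; IA_Fire prints the cooldown and, once it has expired, spawns BP_Missile slightly offset from the Arrow component and resets the timer that Tick counts down.
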(event `self.ReceiveBeginPlay`
  (`EnhancedInputSubsystemInterface.AddMappingContext` (pcsubsystem `EnhancedInputLocalPlayerSubsystem` (`GameplayStatics.GetPlayerController` 0)) "/Game/Input/IMC_PlayerInput.IMC_PlayerInput" 0 (struct)))

(event `self.ReceiveTick`
  (params (DeltaSeconds :type "Float (single-precision)"))
  (set `self.CurrentDelay` (- (`self.CurrentDelay`) DeltaSeconds))
  (`self.K2_SetActorLocation` (+ (* (* (`self.Direction`) (`self.MoveSpeed`)) DeltaSeconds) (`self.K2_GetActorLocation`))))

(event `EnhancedInput|/Game/Input/IA_Move`
  (params (ActionValue :type "Vector2D Structure") (ElapsedSeconds :type "Float (double-precision)") (TriggeredSeconds :type "Float (double-precision)") (InputAction :type "InputAction Object Reference" :default "/Game/Input/IA_Move.IA_Move"))
  (:`Triggered`
    (set `self.Direction` (`KismetMathLibrary.Normal2D` ActionValue) :!label _label))
  (:`Completed`
    (goto _label)))

(event `EnhancedInput|/Game/Input/IA_Fire`
  (params (ActionValue :type Boolean) (ElapsedSeconds :type "Float (double-precision)") (TriggeredSeconds :type "Float (double-precision)") (InputAction :type "InputAction Object Reference" :default "/Game/Input/IA_Fire.IA_Fire"))
  (bind _currentdelay (`self.CurrentDelay`))
  (:`Triggered`
    (`KismetSystemLibrary.PrintString` (`KismetStringLibrary.Conv_DoubleToString` _currentdelay))
    (if (<= _currentdelay 0.0)
      (`|SpawnActorFromClass` "/Game/BluePrint/BP_Missile.BP_Missile_C" (`KismetMathLibrary.Conv_VectorToTransform` (+ (`SceneComponent.K2_GetComponentLocation` (`self.Arrow`)) (10.0 0.0 0.0))) "AlwaysSpawn" "MultiplyWithRoot" null null)
      (set `self.CurrentDelay` (`self.RequireTime`)))))

(fn `UserConstructionScript`)