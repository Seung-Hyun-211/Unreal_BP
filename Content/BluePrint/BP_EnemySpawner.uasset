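; Enemy spawner actor that keeps spawning BP_Enemy at random points marked by its five Arrow components.
; BeginPlay gathers the arrows into an array, and Tick counts down a delay timer that resets to SpawnDelay after each spawn.
; Each spawn picks a random arrow and uses only its world location, so the arrow's rotation and scale are not passed on.
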(event `self.ReceiveBeginPlay`
  (bind _componets (`self.Componets`))
  (`KismetArrayLibrary.Array_Add` _componets (`self.Arrow`))
  (`KismetArrayLibrary.Array_Add` _componets (`self.Arrow1`))
  (`KismetArrayLibrary.Array_Add` _componets (`self.Arrow2`))
  (`KismetArrayLibrary.Array_Add` _componets (`self.Arrow3`))
  (`KismetArrayLibrary.Array_Add` _componets (`self.Arrow4`)))

(event `self.ReceiveTick`
  (params (DeltaSeconds :type "Float (single-precision)"))
  (bind _output_get (set `self.CurrentDelay` (- (`self.CurrentDelay`) DeltaSeconds)))
  (if (<= _output_get 0.0)
    (`|SpawnActorFromClass` "/Game/BluePrint/BP_Enemy.BP_Enemy_C" (`KismetMathLibrary.Conv_VectorToTransform` (`SceneComponent.K2_GetComponentLocation` (`KismetArrayLibrary.Array_Random` (`self.Componets`)))) "Undefined" "MultiplyWithRoot" null null)
    (set `self.CurrentDelay` (`self.SpawnDelay`))))

(fn `UserConstructionScript`)